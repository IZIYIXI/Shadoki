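; Base enemy Blueprint for the garden that grabs fruit when it enters the grab zone.
; An overlap with an actor tagged Fruit stops AI movement and starts a grab, which sets a grabbing flag and plays a montage.
; During the grab it sets the BP_AIController fruit sensing interval to zero, then restores it and clears the flag when a montage notify ends.
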(event OnComponentBeginOverlap(GrabZone)
  (params (OverlappedComponent :type Primitive%20Component%20Object%20Reference) (OtherActor :type Actor%20Object%20Reference) (OtherComp :type Primitive%20Component%20Object%20Reference) (OtherBodyIndex :type Integer) (bFromSweep :type Boolean) (SweepResult :type Hit%20Result%20Structure%20%28by%20ref%29))
  (if (Actor|ActorHasTag OtherActor "Fruit")
    (AI|Navigation|StopMovement (Pawn|GetController))
    (CallFunction|Grab)))

(event Custom|Grab
  (bind _grabmontage (Variables|Default|GetGrabMontage))
  (Variables|Default|SetIsGrabbing true)
  (bind _asbp_aicontroller (Utilities|Casting|CastToBP_AIController (Pawn|GetController)))
  (Class|PawnSensingComponent|SetSensingInterval (Variables|/Game/Garden/Enemies/BP_AIController.BP_AIController_C|GetFruitSensing _asbp_aicontroller) 0.0)
  (Animation|Montage|PlayMontage (Variables|Character|GetMesh) _grabmontage
    (:OnNotifyEnd
      (Animation|StopAnimMontage _grabmontage)
      (Class|PawnSensingComponent|SetSensingInterval (Variables|/Game/Garden/Enemies/BP_AIController.BP_AIController_C|GetFruitSensing _asbp_aicontroller) 0.5)
      (Variables|Default|SetIsGrabbing false))))

(fn ConstructionScript)