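; BP_Fruit_old is a garden fruit pickup that players or enemies collect by touching it.
; On BeginPlay it sets the GrabZone sphere radius to zero, then 100, updating overlaps each time.
; Any overlap plays an explosion sound, before the tag check.
; For Player or Enemy tags, it decrements the current fruit count on its owning BP_PlantBase and destroys itself, doing neither if that owner cast fails.
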(event OnComponentBeginOverlap(GrabZone)
  (params (OverlappedComponent :type Primitive%20Component%20Object%20Reference) (OtherActor :type Actor%20Object%20Reference) (OtherComp :type Primitive%20Component%20Object%20Reference) (OtherBodyIndex :type Integer) (bFromSweep :type Boolean) (SweepResult :type Hit%20Result%20Structure%20%28by%20ref%29))
  (CallFunction|FruitCollected OtherActor))

(event Custom|FruitCollected
  (params (Collector :type Actor%20Object%20Reference))
  ;[1 1 1] Fruit has been collected
  (Audio|PlaySoundatLocation "/Game/StarterContent/Audio/Explosion_Cue.Explosion_Cue" (Transformation|GetActorLocation) "0, 0, 0" 1.0 1.0 0.0 0 0 0)
  (if (Actor|ActorHasTag Collector "Player")
    (bind _asbp_plant_base (Utilities|Casting|CastToBP_PlantBase (Components|GetOwner) :!label _label))
    (Variables|/Game/Garden/Plants/BP_PlantBase.BP_PlantBase_C|SetFruitsNumCurrent _asbp_plant_base (- (Variables|/Game/Garden/Plants/BP_PlantBase.BP_PlantBase_C|GetFruitsNumCurrent _asbp_plant_base) 1))
    (Actor|DestroyActor)
    (elif (Actor|ActorHasTag Collector "Enemy")
      (goto _label))))

(event EventBeginPlay
  (bind _grabzone (Variables|Default|GetGrabZone))
  (Components|Sphere|SetSphereRadius _grabzone 0.0 true)
  (Components|Sphere|SetSphereRadius _grabzone 1e+02 true))

(fn ConstructionScript)