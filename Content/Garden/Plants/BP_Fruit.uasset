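; BP_Fruit is a collectible garden fruit that scores a point for the player or the enemy who grabs it.
; The first non-fruit overlap destroys its GrabZone to block retriggering, then collection runs after a short delay and plays an explosion cue.
; The collector's actor tag picks which TopDownGameMode score rises.
; It then refreshes the score UI, decrements the owning BP_PlantBase's fruit count, leaves the game mode's Fruits list and destroys itself.
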(event OnComponentBeginOverlap(GrabZone)
  (params (OverlappedComponent :type Primitive%20Component%20Object%20Reference) (OtherActor :type Actor%20Object%20Reference) (OtherComp :type Primitive%20Component%20Object%20Reference) (OtherBodyIndex :type Integer) (bFromSweep :type Boolean) (SweepResult :type Hit%20Result%20Structure%20%28by%20ref%29))
  ;[1 1 1] Initiating fruit collection
  (if (not (Actor|ActorHasTag OtherActor "Fruit"))
    (Components|DestroyComponent (Variables|Default|GetGrabZone))
    (Utilities|FlowControl|Delay 0.444444)
    (CallFunction|FruitCollected OtherActor)))

(event Custom|FruitCollected
  (params (Collector :type Actor%20Object%20Reference))
  ;[1 1 1] Fruit has been collected
  (Audio|PlaySoundatLocation "/Game/StarterContent/Audio/Explosion_Cue.Explosion_Cue" (Transformation|GetActorLocation) "0, 0, 0" 1.0 1.0 0.0 0 0 0)
  (bind _astop_down_game_mode (Utilities|Casting|CastToTopDownGameMode (Game|GetGameMode)))
  (if (Actor|ActorHasTag Collector "Player")
    (Math|Integer|IncrementInt (Variables|/Game/TopDownBP/Blueprints/TopDownGameMode.TopDownGameMode_C|GetPlayerScore _astop_down_game_mode)
      (:%20%20
        (bind _astop_down_character (Utilities|Casting|CastToTopDownCharacter (Game|GetPlayerCharacter 0) :!label _label))
        (Default|UpdateScores (Variables|/Game/TopDownBP/Blueprints/TopDownCharacter.TopDownCharacter_C|GetPlayerUI _astop_down_character))
        (bind _asbp_plant_base (Utilities|Casting|CastToBP_PlantBase (Components|GetOwner)))
        (Math|Integer|DecrementInt (Variables|/Game/Garden/Plants/BP_PlantBase.BP_PlantBase_C|GetFruitsNumCurrent _asbp_plant_base)
          (:%20%20
            (bind _astop_down_game_mode_2 (Utilities|Casting|CastToTopDownGameMode (Game|GetGameMode)))
            (Utilities|Array|RemoveItem (Variables|/Game/TopDownBP/Blueprints/TopDownGameMode.TopDownGameMode_C|GetFruits _astop_down_game_mode_2) self)
            (Actor|DestroyActor)))))
    (elif (Actor|ActorHasTag Collector "Enemy")
      (Math|Integer|IncrementInt (Variables|/Game/TopDownBP/Blueprints/TopDownGameMode.TopDownGameMode_C|GetEnemyScore _astop_down_game_mode)
        (:%20%20
          (goto _label))))))

(fn ConstructionScript)