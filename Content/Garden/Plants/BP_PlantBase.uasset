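; Base garden plant that periodically grows fruit up to a randomized capacity.
; On BeginPlay it rolls fruit capacity and growth time, scaling its width with capacity and its height inversely with growth time.
; A looping timer spawns BP_Fruit at FruitSpawner, spreading roll angles evenly over a full turn at a fixed pitch.
; Each fruit is registered in TopDownGameMode's Fruits array, followed by a sound.
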(event Custom|GrowFruit
  (bind _fruitsnummax (Variables|Fruits|GetFruitsNumMax))
  (bind _fruitsnumcurrent (Variables|Fruits|GetFruitsNumCurrent))
  ;[1 1 1] Fruits growing
  (if (< _fruitsnumcurrent _fruitsnummax)
    (bind _returnvalue (Game|SpawnActorfromClass "/Game/Garden/Plants/BP_Fruit.BP_Fruit_C" (Math|Transform|MakeTransform (Transformation|GetWorldLocation (Variables|Default|GetFruitSpawner)) (Math|Rotator|MakeRotator (* _fruitsnumcurrent (/ 3.6e+02 (Math|Conversions|ToFloat(Integer) _fruitsnummax))) -45.0 0.0)) "AlwaysSpawn" self 0))
    (bind _astop_down_game_mode (Utilities|Casting|CastToTopDownGameMode (Game|GetGameMode)))
    (Utilities|Array|Add (Variables|/Game/TopDownBP/Blueprints/TopDownGameMode.TopDownGameMode_C|GetFruits _astop_down_game_mode) _returnvalue)
    (Math|Integer|IncrementInt (Variables|Fruits|GetFruitsNumCurrent)
      (:%20%20
        (Audio|PlaySoundatLocation "/Game/StarterContent/Audio/Collapse_Cue.Collapse_Cue" (Transformation|GetActorLocation) "0, 0, 0" 1.0 1.0 0.0 0 0 0)))))

(event EventBeginPlay
  (bind _plantbody (Variables|Default|GetPlantBody))
  (bind _returnvalue (Transformation|GetWorldScale _plantbody))
  ;[1 1 1] Setting up growth parameters
  (Utilities|FlowControl|Sequence
    (:then_0
      (bind _output_get (Variables|Fruits|SetFruitsNumMax (Math|Random|RandomIntegerinRange 1 16)))
      (Transformation|SetActorScale3D (Math|Vector|MakeVector (/ (Math|Conversions|ToFloat(Integer) _output_get) 8.0) (/ (Math|Conversions|ToFloat(Integer) _output_get) 8.0) (.z (Transformation|GetWorldScale _plantbody)))))
    (:then_1
      (bind _output_get_2 (Variables|Fruits|SetFruitGrowthTime (Math|Random|RandomFloatinRange 8.0 16.0)))
      (Transformation|SetActorScale3D (Math|Vector|MakeVector (.x _returnvalue) (.y _returnvalue) (/ 12.0 _output_get_2))))
    (:then_2
      (Utilities|Time|SetTimerbyEvent (delegate Custom|GrowFruit) _output_get_2 true))))

(fn ConstructionScript)